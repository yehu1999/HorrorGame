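; Global function library with shortcuts to the game instance, player character, controller and character state, plus save/load helpers for settings and player profiles.
; Settings sync between the game instance and their own save slot, while the active profile's slot stores player data and per-map level records.
; Level loading snapshots and destroys placed items and equipment, returning the saved record if one exists.
; Level saving writes back the game instance's current level data.
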(fn GetBPGameInstance
  (bind _asbp_game_instance (Utilities|Casting|CastToBP_GameInstance (Game|GetGameInstance)))
  (return _asbp_game_instance))

(fn GetBPCharacter
  (bind _asbp_character (Utilities|Casting|CastToBP_Character (Game|Player|GetPlayerPawn 0)))
  (return _asbp_character))

(fn GetBPPlayerController
  (bind _asbp_player_controller (Utilities|Casting|CastToBP_PlayerController (Game|GetPlayerController 0)))
  (return _asbp_player_controller))

(fn GetCharacterPlayerState
  (bind _e_playerstate (Default|GetCharacterPlayerState (Get|GetBPCharacter)))
  (return _e_playerstate))

(fn HideActorwithAttached
  (params (Actor :type Actor%20Object%20Reference) (bNewHidden :type Boolean))
  (Rendering|SetActorHiddenInGame Actor bNewHidden)
  (for _array_element (Actor|GetAttachedActors Actor true false)
    (Rendering|SetActorHiddenInGame _array_element bNewHidden)))

(fn SetCharacterPlayerState
  (params (E_PlayerState :type E_PlayerState%20Enum :default "NewEnumerator2"))
  (Default|SetCharacterPlayerState (Get|GetBPCharacter) E_PlayerState))

(fn SearchLevelProfile
  (params (Array :type Array%20of%20S%20Level%20SG%20Structures))
  (bind (_array_element _array_index) (Utilities|Array|ForEachLoopwithBreak Array)
    (:LoopBody
      (bind _returnvalue (Game|GetCurrentLevelName 0))
      (if (Utilities|Enum|Equal(Enum) _returnvalue (Utilities|Struct|BreakS_Level_SG _array_element))
        (return true _array_index)))
    (:Completed
      (return false -1))))

(fn DetectLevel
  (params (Is_DestoryActors :type Boolean))
  (Utilities|FlowControl|Sequence
    (:then_0
      (bind _outactors (Actor|GetAllActorsOfClass 0 "/Game/Game/Blueprints/Objects/BP_Item.BP_Item_C"))
      (for (_array_element _array_index) _outactors
        (Utilities|Array|Add (LocalVariables|GetLocal_Array_Item) (Utilities|Struct|MakeS_Item_SG (Utilities|String|Append "Item_" (Utilities|String|ToString(Integer) _array_index)) (Transformation|GetActorTransform _array_element) (Variables|/Game/Game/Blueprints/Objects/BP_Object.BP_Object_C|GetInventoryContent _array_element)))
        (if Is_DestoryActors
          (Actor|DestroyActor _array_element))))
    (:then_1
      (bind _outactors_2 (Actor|GetAllActorsOfClass 0 "/Game/Game/Blueprints/Objects/BP_Equipment.BP_Equipment_C"))
      (for (_array_element_2 _array_index_2) _outactors_2
        (Utilities|Array|Add (LocalVariables|GetLocal_Array_Equipment) (Utilities|Struct|MakeS_Equipment_SG (Utilities|String|Append "Equipment_" (Utilities|String|ToString(Integer) _array_index_2)) (Transformation|GetActorTransform _array_element_2) (Variables|/Game/Game/Blueprints/Objects/BP_Object.BP_Object_C|GetInventoryContent _array_element_2)))
        (if Is_DestoryActors
          (Actor|DestroyActor _array_element_2)))
      (bind _returnvalue (Game|GetCurrentLevelName 0))
      (return (Utilities|Struct|MakeS_Level_SG _returnvalue (LocalVariables|GetLocal_Array_Item) (LocalVariables|GetLocal_Array_Equipment))))))

(fn GetActivePlayerProfile
  (bind _bp_game_instance (Get|GetBPGameInstance))
  (return (Utilities|Array|Get(acopy) (Variables|/Game/Game/Blueprints/BP_GameInstance.BP_GameInstance_C|GetPlayerProfile_Array _bp_game_instance) (Variables|/Game/Game/Blueprints/BP_GameInstance.BP_GameInstance_C|GetPlayerProfile_Index _bp_game_instance))))

(fn CreateNewPlayerProfile
  (bind _bp_game_instance (Get|GetBPGameInstance))
  (bind _playerprofile_array (Variables|/Game/Game/Blueprints/BP_GameInstance.BP_GameInstance_C|GetPlayerProfile_Array _bp_game_instance))
  (Default|SearchPlayerProfile _bp_game_instance)
  (bind _returnvalue (Utilities|Array|AddUnique _playerprofile_array (Utilities|String|Append (LocalVariables|GetLocal_PlayerProfileSlot_Base) "_" (Utilities|String|ToString(Integer) (Utilities|Array|Length _playerprofile_array)))))
  (Utilities|Array|Swap _playerprofile_array _returnvalue))

(fn IsPalyerProfileExisted
  (bind _bp_game_instance (Get|GetBPGameInstance))
  (Default|SearchPlayerProfile _bp_game_instance)
  (if (Utilities|Array|IsNotEmpty (Variables|/Game/Game/Blueprints/BP_GameInstance.BP_GameInstance_C|GetPlayerProfile_Array _bp_game_instance))
    (return true)
    (else
      (return false))))

(fn LoadSettingProfile
  (bind _bp_game_instance (Get|GetBPGameInstance))
  (bind _bp_game_instance_2 (Get|GetBPGameInstance))
  (bind _returnvalue (SaveGame|DoesSaveGameExist (LocalVariables|GetLocal_SlotString)))
  (if _returnvalue
    (bind _returnvalue_2 (SaveGame|LoadGamefromSlot (LocalVariables|GetLocal_SlotString)))
    (bind _asbp_save_game_profile_setting (Utilities|Casting|CastToBP_SaveGameProfile_Setting _returnvalue_2))
    (Variables|/Game/Game/Blueprints/BP_GameInstance.BP_GameInstance_C|SetS_SoundSetting_Player _bp_game_instance_2 (Variables|/Game/Game/Blueprints/BP_SaveGameProfile_Setting.BP_SaveGameProfile_Setting_C|GetS_SoundSetting_Player _asbp_save_game_profile_setting))
    (Variables|/Game/Game/Blueprints/BP_GameInstance.BP_GameInstance_C|SetS_VedioSetting_Player _bp_game_instance_2 (Variables|/Game/Game/Blueprints/BP_SaveGameProfile_Setting.BP_SaveGameProfile_Setting_C|GetS_VedioSetting_Player _asbp_save_game_profile_setting))
    (Variables|/Game/Game/Blueprints/BP_GameInstance.BP_GameInstance_C|SetS_TextSetting_Player _bp_game_instance_2 (Variables|/Game/Game/Blueprints/BP_SaveGameProfile_Setting.BP_SaveGameProfile_Setting_C|GetS_TextSetting_Player _asbp_save_game_profile_setting))
    (else
      (bind _returnvalue_3 (SaveGame|CreateSaveGameObject "/Game/Game/Blueprints/BP_SaveGameProfile_Setting.BP_SaveGameProfile_Setting_C"))
      (Variables|/Game/Game/Blueprints/BP_SaveGameProfile_Setting.BP_SaveGameProfile_Setting_C|SetS_SoundSetting_Player _returnvalue_3 (Variables|/Game/Game/Blueprints/BP_GameInstance.BP_GameInstance_C|GetS_SoundSetting_Player _bp_game_instance))
      (Variables|/Game/Game/Blueprints/BP_SaveGameProfile_Setting.BP_SaveGameProfile_Setting_C|SetS_VedioSetting_Player _returnvalue_3 (Variables|/Game/Game/Blueprints/BP_GameInstance.BP_GameInstance_C|GetS_VedioSetting_Player _bp_game_instance))
      (Variables|/Game/Game/Blueprints/BP_SaveGameProfile_Setting.BP_SaveGameProfile_Setting_C|SetS_TextSetting_Player _returnvalue_3 (Variables|/Game/Game/Blueprints/BP_GameInstance.BP_GameInstance_C|GetS_TextSetting_Player _bp_game_instance))
      (SaveGame|SaveGametoSlot _returnvalue_3 (LocalVariables|GetLocal_SlotString)))))

(fn SaveSettingProfile
  (bind _bp_game_instance (Get|GetBPGameInstance))
  (bind _local_slotstring (LocalVariables|GetLocal_SlotString))
  (bind _returnvalue (SaveGame|DoesSaveGameExist (LocalVariables|GetLocal_SlotString)))
  (if _returnvalue
    (bind _returnvalue_2 (SaveGame|LoadGamefromSlot (LocalVariables|GetLocal_SlotString)))
    (bind _asbp_save_game_profile_setting (Utilities|Casting|CastToBP_SaveGameProfile_Setting _returnvalue_2))
    (Variables|/Game/Game/Blueprints/BP_SaveGameProfile_Setting.BP_SaveGameProfile_Setting_C|SetS_SoundSetting_Player _asbp_save_game_profile_setting (Variables|/Game/Game/Blueprints/BP_GameInstance.BP_GameInstance_C|GetS_SoundSetting_Player _bp_game_instance))
    (Variables|/Game/Game/Blueprints/BP_SaveGameProfile_Setting.BP_SaveGameProfile_Setting_C|SetS_VedioSetting_Player _asbp_save_game_profile_setting (Variables|/Game/Game/Blueprints/BP_GameInstance.BP_GameInstance_C|GetS_VedioSetting_Player _bp_game_instance))
    (Variables|/Game/Game/Blueprints/BP_SaveGameProfile_Setting.BP_SaveGameProfile_Setting_C|SetS_TextSetting_Player _asbp_save_game_profile_setting (Variables|/Game/Game/Blueprints/BP_GameInstance.BP_GameInstance_C|GetS_TextSetting_Player _bp_game_instance))
    (SaveGame|SaveGametoSlot _asbp_save_game_profile_setting _local_slotstring)
    ;[1 1 1] 注释
    (Development|PrintString 0 (Utilities|String|Append _local_slotstring ":" "Save"))))

(fn LoadPlayerProfilePlayer
  (params (Is_Create_NewProfile :type Boolean))
  (if Is_Create_NewProfile
    (保存游戏|CreateNewPlayerProfile))
  (bind _output_get (LocalVariables|SetLocal_SlotString (保存游戏|GetActivePlayerProfile)))
  (bind _returnvalue (SaveGame|DoesSaveGameExist _output_get))
  (if _returnvalue
    (bind _returnvalue_2 (SaveGame|LoadGamefromSlot (LocalVariables|GetLocal_SlotString)))
    (bind _asbp_save_game_profile_player (Utilities|Casting|CastToBP_SaveGameProfile_Player _returnvalue_2))
    (SaveGame|SaveGametoSlot _asbp_save_game_profile_player (LocalVariables|GetLocal_SlotString))
    (return _asbp_save_game_profile_player)
    (else
      (bind _returnvalue_3 (SaveGame|CreateSaveGameObject "/Game/Game/Blueprints/BP_SaveGameProfile_Player.BP_SaveGameProfile_Player_C"))
      (SaveGame|SaveGametoSlot _returnvalue_3 (LocalVariables|GetLocal_SlotString))
      (return _returnvalue_3))))

(fn SavePlayerProfilePlayer
  (params (S_Player :type S%20Player%20SG%20Structure))
  (bind _output (保存游戏|GetActivePlayerProfile))
  (bind _returnvalue (SaveGame|DoesSaveGameExist _output))
  (if _returnvalue
    (bind _returnvalue_2 (SaveGame|LoadGamefromSlot _output))
    (bind _asbp_save_game_profile_player (Utilities|Casting|CastToBP_SaveGameProfile_Player _returnvalue_2))
    (Variables|/Game/Game/Blueprints/BP_SaveGameProfile_Player.BP_SaveGameProfile_Player_C|SetS_Player _asbp_save_game_profile_player S_Player)
    (Variables|/Game/Game/Blueprints/BP_SaveGameProfile_Player.BP_SaveGameProfile_Player_C|SetIs_FirstLoad _asbp_save_game_profile_player false)
    (SaveGame|SaveGametoSlot _asbp_save_game_profile_player _output)
    ;[1 1 1] 注释
    (Development|PrintString 0 (Utilities|String|Append "Save To Player: " _output))))

(fn LoadPlayerProfileLevel
  (LocalVariables|SetLocal_PlayerProfile_SlotString (保存游戏|GetActivePlayerProfile))
  (bind _returnvalue (SaveGame|LoadGamefromSlot (LocalVariables|GetLocal_PlayerProfile_SlotString)))
  (bind _asbp_save_game_profile_player (Utilities|Casting|CastToBP_SaveGameProfile_Player _returnvalue))
  (bind (_is_found _index) (保存游戏|SearchLevelProfile 0 (Variables|/Game/Game/Blueprints/BP_SaveGameProfile_Player.BP_SaveGameProfile_Player_C|GetArray_Level _asbp_save_game_profile_player)))
  (if _is_found
    (SaveGame|DetectLevel true)
    (return (Utilities|Array|Get(acopy) (Variables|/Game/Game/Blueprints/BP_SaveGameProfile_Player.BP_SaveGameProfile_Player_C|GetArray_Level _asbp_save_game_profile_player) _index))
    (else
      (bind _s_level (SaveGame|DetectLevel true))
      (Utilities|Array|Add (Variables|/Game/Game/Blueprints/BP_SaveGameProfile_Player.BP_SaveGameProfile_Player_C|GetArray_Level _asbp_save_game_profile_player) _s_level)
      (SaveGame|SaveGametoSlot _asbp_save_game_profile_player (LocalVariables|GetLocal_PlayerProfile_SlotString))
      (return _s_level))))

(fn SavePlayerProfileLevel
  (bind _output (保存游戏|GetActivePlayerProfile))
  (bind _bp_game_instance (Get|GetBPGameInstance))
  (bind _current_level_sg (Variables|/Game/Game/Blueprints/BP_GameInstance.BP_GameInstance_C|GetCurrent_Level_SG _bp_game_instance))
  (bind (_array_item _array_equipment) (Utilities|Struct|BreakS_Level_SG _current_level_sg))
  (bind _returnvalue (SaveGame|LoadGamefromSlot _output))
  (bind _asbp_save_game_profile_player (Utilities|Casting|CastToBP_SaveGameProfile_Player _returnvalue))
  (bind _index (保存游戏|SearchLevelProfile 0 (Variables|/Game/Game/Blueprints/BP_SaveGameProfile_Player.BP_SaveGameProfile_Player_C|GetArray_Level _asbp_save_game_profile_player)))
  (Utilities|Struct|SetmembersinS_Level_SG (Utilities|Array|Get(acopy) (Variables|/Game/Game/Blueprints/BP_SaveGameProfile_Player.BP_SaveGameProfile_Player_C|GetArray_Level _asbp_save_game_profile_player) _index) _array_item _array_equipment)
  (SaveGame|SaveGametoSlot _asbp_save_game_profile_player _output)
  ;[1 1 1] 注释
  (Development|PrintString 0 (Utilities|String|Append "Save To Level: " _output)))