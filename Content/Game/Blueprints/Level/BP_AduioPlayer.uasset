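; BP_AduioPlayer is a level Blueprint actor that plays a sound at its location with timed, localized subtitles.
; The construction script gathers rows matching its sound from the Chinese and English subtitle DataTables, using the Chinese table's row names for both.
; Play_Aduio starts the sound, then steps through lines on the character's subtitle widget, rechecking the language setting and waiting each line's duration.
; After the last line it resets and hides the subtitle.
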(event Custom|Play_Aduio
  (bind _bp_character (CallFunction|GetBPCharacter))
  (bind _ac_ui (Variables|/Game/Game/Blueprints/BP_Character.BP_Character_C|GetAC_UI _bp_character))
  (bind _wb_subtitle (Variables|/Game/Game/Blueprints/Components/AC_UI_Character.AC_UI_Character_C|GetWB_Subtitle _ac_ui))
  (Audio|PlaySoundatLocation (Variables|Default|GetAduio) (Transformation|GetActorLocation) "0, 0, 0" 1.0 1.0 0.0 0 0 0 0)
  (switch Utilities|FlowControl|Switch|SwitchonE_Language (Utilities|Struct|BreakS_TextSetting (Variables|/Game/Game/Blueprints/BP_GameInstance.BP_GameInstance_C|GetS_TextSetting_Player (CallFunction|GetBPGameInstance))) :!label _label
    (:NewEnumerator0
      (Variables|Default|SetArray_Subtitle (Variables|Default|GetArray_Subtitle_CN)))
    (:NewEnumerator1
      (Variables|Default|SetArray_Subtitle (Variables|Default|GetArray_Subtitle_EN))))
  (Default|ShowSubtitle _wb_subtitle (Utilities|Array|Get(acopy) (Variables|Default|GetArray_Subtitle) (Variables|Default|GetPlayIndex)))
  (Utilities|FlowControl|Delay (Utilities|Struct|BreakS_Subtitle (Utilities|Array|Get(acopy) (Variables|Default|GetArray_Subtitle) (Variables|Default|GetPlayIndex))))
  (bind _result (Math|Integer|IncrementInt (Variables|Default|GetPlayIndex))
    (:%20%20
      (if (>= _result (Utilities|Array|Length (Variables|Default|GetArray_Subtitle)))
        (Variables|Default|SetPlayIndex 0)
        (Default|HideSubtitle _wb_subtitle)
        (else
          (goto _label))))))

(event EventBeginPlay)

(event EventTick
  (params (DeltaSeconds :type Float%20%28single-precision%29)))

(fn ConstructionScript
  (bind _outrownames (DataTable|GetDataTableRowNames "/Game/Game/Data/Subtitle/DT_Subtitle.DT_Subtitle"))
  (for _array_element _outrownames
    (Utilities|FlowControl|Sequence
      (:then_0
        (bind _returnvalue (Utilities|GetDataTableRow "/Game/Game/Data/Subtitle/DT_Subtitle.DT_Subtitle" _array_element)
          (:then
            (if (== (Variables|Default|GetAduio) (Utilities|Struct|BreakS_Subtitle _returnvalue))
              (Utilities|Array|AddUnique (Variables|Default|GetArray_Subtitle_CN) _returnvalue)))))
      (:then_1
        (bind _returnvalue_2 (Utilities|GetDataTableRow "/Game/Game/Data/Subtitle/Translations/DT_Subtitle_EN.DT_Subtitle_EN" _array_element)
          (:then
            (if (== (Variables|Default|GetAduio) (Utilities|Struct|BreakS_Subtitle _returnvalue_2))
              (Utilities|Array|AddUnique (Variables|Default|GetArray_Subtitle_EN) _returnvalue_2))))))))