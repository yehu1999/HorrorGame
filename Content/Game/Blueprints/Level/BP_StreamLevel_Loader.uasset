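; BP_StreamLevel_Loader is a trigger actor that swaps streamed levels when BP_Character overlaps it.
; It optionally shows a game-instance loading screen, loads LevelToLoad without blocking, then after a short delay hides the screen and unloads LevelToUnload.
; An optional teleport to TeleportPoint's arrow runs without waiting for the load, also setting control rotation.
; The unloaded level should not be the one containing this loader.
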(event EventBeginPlay)

(event Collision|EventActorBeginOverlap
  (params (OtherActor :type Actor%20Object%20Reference))
  (bind _teleportpoint (Variables|关卡|GetTeleportPoint))
  (bind _arrow (Variables|/Game/Game/Blueprints/Level/BP_TeleportPoint.BP_TeleportPoint_C|GetArrow _teleportpoint))
  (bind _asbp_character (Utilities|Casting|CastToBP_Character OtherActor))
  (Utilities|FlowControl|Sequence
    (:then_0
      (if (Variables|关卡|GetIs_Show_LoadingScreen)
        (Default|UIShowLoadingScreen (CallFunction|GetBPGameInstance) true (Variables|关卡|GetLoadingScreen_MediaSource))))
    (:then_1
      (bind _level_toload (Variables|Levels|GetLevel_ToLoad)
        (:then
          (Class|GameplayStatics|LoadStreamLevelbySoftObjectPtr _level_toload true false)
          (Utilities|FlowControl|Delay 2.0)
          (Default|UIShowLoadingScreen (CallFunction|GetBPGameInstance) false)
          ;[1 1 1] 被Unload的关卡不应该是该LevelLoader所在的关卡
          (bind _level_tounload (Variables|Levels|GetLevel_ToUnload)
            (:then
              (Class|GameplayStatics|UnloadStreamLevelbySoftObjectPtr _level_tounload false))
            (:else)))
        (:else)))
    (:then_2
      (if (Variables|Levels|GetIs_Teleport)
        (Transformation|Teleport _asbp_character (Transformation|GetWorldLocation _arrow) "0, 0, 0")
        (Pawn|SetControlRotation (Game|GetPlayerController 0) (Transformation|GetWorldRotation _arrow))))))

(event EventTick
  (params (DeltaSeconds :type Float%20%28single-precision%29)))

(fn ConstructionScript)