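; BP_Area_CharacterChanger is a level trigger area that toggles the player character's unarmed equipment state.
; Its Box begin and end overlap events check that the other actor is the character returned by GetBPCharacter.
; They then call EquipmentUnarm on that character's ACInventoryEquipment component, passing true on entry and false on exit.
; Despite the name, the graph contains no character-swapping logic.
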(event OnComponentBeginOverlap(Box)
  (params (OverlappedComponent :type Primitive%20Component%20Object%20Reference) (OtherActor :type Actor%20Object%20Reference) (OtherComp :type Primitive%20Component%20Object%20Reference) (OtherBodyIndex :type Integer) (bFromSweep :type Boolean) (SweepResult :type Hit%20Result%20Structure%20%28by%20ref%29))
  (bind _bp_character (CallFunction|GetBPCharacter))
  (if (== OtherActor _bp_character)
    (Default|EquipmentUnarm (Variables|/Game/Game/Blueprints/BP_Character.BP_Character_C|GetAC_Inventory_Equipment _bp_character) true)))

(event OnComponentEndOverlap(Box)
  (params (OverlappedComponent :type Primitive%20Component%20Object%20Reference) (OtherActor :type Actor%20Object%20Reference) (OtherComp :type Primitive%20Component%20Object%20Reference) (OtherBodyIndex :type Integer))
  (bind _bp_character (CallFunction|GetBPCharacter))
  (if (== OtherActor _bp_character)
    (Default|EquipmentUnarm (Variables|/Game/Game/Blueprints/BP_Character.BP_Character_C|GetAC_Inventory_Equipment _bp_character) false)))

(event EventBeginPlay)

(event Collision|EventActorBeginOverlap
  (params (OtherActor :type Actor%20Object%20Reference)))

(event EventTick
  (params (DeltaSeconds :type Float%20%28single-precision%29)))

(fn ConstructionScript)