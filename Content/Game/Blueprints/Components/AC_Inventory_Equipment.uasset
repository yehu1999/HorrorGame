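; Actor component that manages the player's handheld equipment inventory: flashlight, candle and camera.
; On BeginPlay it caches the three items from tagged child actor components on its owner.
; Unlocking adds to a unique list and saves the player profile; selecting an unlocked item toggles it, unequipping all others first.
; Equip, use and unequip calls route by active row name to each item's InHandable component.
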(event Custom|Change_Equipment
  (params (RowName_PlayerEquipment%20 :type Name))
  ;[1 1 1] Equipment
  (if (CallFunction|IsEquipmentUnlocked RowName_PlayerEquipment%20)
    (if (!= (Variables|Default|GetRowName_ActiveEquipment) RowName_PlayerEquipment%20)
      (Variables|Default|SetRowName_ActiveEquipment RowName_PlayerEquipment%20)
      (else
        (Variables|Default|SetRowName_ActiveEquipment "None")))
    (switch name (Variables|Default|GetRowName_ActiveEquipment)
      (:None
        (CallFunction|UnequipAll))
      (:Flashlight
        (CallFunction|UnequipAll)
        (Default|CallEquip (Variables|/Game/Game/Blueprints/InHands/BP_FlashLight.BP_FlashLight_C|GetAC_InHandable (Variables|Default|GetBP_FlashLight))))
      (:Candle
        (CallFunction|UnequipAll)
        (Default|CallEquip (Variables|/Game/Game/Blueprints/InHands/BP_Candle.BP_Candle_C|GetAC_InHandable (Variables|Default|GetBP%20Candle))))
      (:Camera
        (CallFunction|UnequipAll)
        (Default|CallEquip (Variables|/Game/Game/Blueprints/InHands/BP_Camera.BP_Camera_C|GetAC_InHandable (Variables|Default|GetBP%20Camera)))))))

(event Custom|Use_Equipment
  ;[1 1 1] Equipment
  (switch name (Variables|Default|GetRowName_ActiveEquipment)
    (:Flashlight
      (Default|CallUse (Variables|/Game/Game/Blueprints/InHands/BP_FlashLight.BP_FlashLight_C|GetAC_InHandable (Variables|Default|GetBP_FlashLight))))
    (:Candle
      (Default|CallUse (Variables|/Game/Game/Blueprints/InHands/BP_Candle.BP_Candle_C|GetAC_InHandable (Variables|Default|GetBP%20Candle))))
    (:Camera
      (Default|CallUse (Variables|/Game/Game/Blueprints/InHands/BP_Camera.BP_Camera_C|GetAC_InHandable (Variables|Default|GetBP%20Camera))))))

(event Custom|Add_New_Equipment
  (params (NewEquipment :type Name))
  (Utilities|Array|AddUnique (Variables|Default|GetUnlocked_Equipments) NewEquipment)
  (Default|CharacterSaveGamePlayerProfile (CallFunction|GetBPCharacter)))

(event Custom|Unequip_All
  ;[1 1 1] Equipment
  (Default|CallUnequip (Variables|/Game/Game/Blueprints/InHands/BP_FlashLight.BP_FlashLight_C|GetAC_InHandable (Variables|Default|GetBP_FlashLight)))
  (Default|CallUnequip (Variables|/Game/Game/Blueprints/InHands/BP_Candle.BP_Candle_C|GetAC_InHandable (Variables|Default|GetBP%20Candle)))
  (Default|CallUnequip (Variables|/Game/Game/Blueprints/InHands/BP_Camera.BP_Camera_C|GetAC_InHandable (Variables|Default|GetBP%20Camera))))

(event EventBeginPlay
  (bind _asbp_flash_light (Utilities|Casting|CastToBP_FlashLight (Variables|/Script/Engine.ChildActorComponent|GetChildActor (Utilities|Array|Get(acopy) (Actor|GetComponentsbyTag (Components|GetOwner) "/Script/Engine.ChildActorComponent" "FlashLight")))))
  (Variables|Default|SetBP_FlashLight _asbp_flash_light)
  (bind _asbp_candle (Utilities|Casting|CastToBP_Candle (Variables|/Script/Engine.ChildActorComponent|GetChildActor (Utilities|Array|Get(acopy) (Actor|GetComponentsbyTag (Components|GetOwner) "/Script/Engine.ChildActorComponent" "Candle")))))
  (Variables|Default|SetBP%20Candle _asbp_candle)
  (bind _asbp_camera (Utilities|Casting|CastToBP_Camera (Variables|/Script/Engine.ChildActorComponent|GetChildActor (Utilities|Array|Get(acopy) (Actor|GetComponentsbyTag (Components|GetOwner) "/Script/Engine.ChildActorComponent" "Camera")))))
  (Variables|Default|SetBP%20Camera _asbp_camera))

(fn IsEquipmentUnlocked
  (params (Equipment :type Name%20%28by%20ref%29))
  (return (>= (Utilities|Array|FindItem (Variables|Default|GetUnlocked_Equipments) Equipment) 0)))