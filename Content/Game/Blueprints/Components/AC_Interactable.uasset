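; AC_Interactable is an actor component that gives its owner a hint widget for interaction.
; On BeginPlay it spawns a BP_WidgetActor and attaches it to the "Hint" socket of the owner's static mesh, keeping world rotation and scale.
; Show_Hint makes the widget visible and hides it after a short retriggerable delay, so repeated calls keep it on screen.
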(event Custom|Show_Hint
  (bind _bp_widgetactor (Variables|Default|GetBP_WidgetActor))
  (Default|SetVisibility _bp_widgetactor true)
  (Utilities|FlowControl|RetriggerableDelay 0.2)
  (Default|SetVisibility _bp_widgetactor false))

(event EventBeginPlay
  (bind _returnvalue (Components|GetOwner))
  (bind _returnvalue_2 (Game|SpawnActorfromClass "/Game/Game/UI/InGame/BP_WidgetActor.BP_WidgetActor_C" (Math|Transform|MakeTransform (Transformation|GetActorLocation _returnvalue)) "AlwaysSpawn" "MultiplyWithRoot" 0 0))
  (bind _output_get (Variables|Default|SetBP_WidgetActor _returnvalue_2))
  (Transformation|AttachComponentToComponent _output_get (Actor|GetComponentbyClass _returnvalue "/Script/Engine.StaticMeshComponent") "Hint" "SnapToTarget" "KeepWorld" "KeepWorld" true))