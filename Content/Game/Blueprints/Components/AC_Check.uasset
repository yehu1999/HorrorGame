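; Component for inspecting world objects up close, with rotate, zoom and take actions.
; CheckObject toggles inspection of the actor detected by AC_Interact, switching player state and calling its AC_Checkable, with one-second delay flags blocking rapid re-toggling.
; Rotation and clamped scaling act on the character's ChildActorCheckingObject, and RestoreCharacter resets both along with player state.
; Take_Object restores the character, then triggers the inspected actor's AC_Interactable interaction.
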(event Custom|Rotate_CheckingObject
  (params (X%20%28Roll%29 :type Float%20%28single-precision%29) (Y%20%28Pitch%29 :type Float%20%28single-precision%29))
  (bind _bp_character (CallFunction|GetBPCharacter))
  (bind _childactor_checkingobject (Variables|/Game/Game/Blueprints/BP_Character.BP_Character_C|GetChildActor_CheckingObject _bp_character))
  (bind _relativerotation (Variables|/Script/Engine.SceneComponent|GetRelativeRotation _childactor_checkingobject))
  (Transformation|SetRelativeRotation _childactor_checkingobject (Math|Rotator|CombineRotators _relativerotation (Math|Rotator|MakeRotator X%20%28Roll%29 0.0 0.0)) false false)
  (Transformation|SetRelativeRotation _childactor_checkingobject (Math|Rotator|CombineRotators _relativerotation (Math|Rotator|MakeRotator 0.0 Y%20%28Pitch%29 0.0)) false false))

(event Custom|Scale_CheckingObject
  (params (Delta :type Float%20%28double-precision%29))
  (bind _bp_character (CallFunction|GetBPCharacter))
  (bind _childactor_checkingobject (Variables|/Game/Game/Blueprints/BP_Character.BP_Character_C|GetChildActor_CheckingObject _bp_character))
  (Transformation|SetRelativeScale3D _childactor_checkingobject (Math|Vector|ClampVectorSize (+ (Variables|/Script/Engine.SceneComponent|GetRelativeScale3D _childactor_checkingobject) (* Delta 0.2)) 1.0 5.0)))

(event Custom|Take_Object
  (CallFunction|RestoreCharacter)
  (bind _checking_actor (Variables|Default|GetChecking_Actor)
    (:then
      (Default|CallOnInteract (Actor|GetComponentbyClass _checking_actor "/Game/Game/Blueprints/Components/AC_Interactable.AC_Interactable_C")))
    (:else)))

(event Custom|CheckObject
  (bind _checking_actor (Variables|Default|GetChecking_Actor)
    (:then
      (if (and (not (Variables|Default|GetIs_EndChecking)) (not (Variables|Default|GetIs_StartChecking)))
        (Variables|Default|SetIs_EndChecking true)
        (Default|EndChecking (Actor|GetComponentbyClass _checking_actor "/Game/Game/Blueprints/Components/AC_Checkable.AC_Checkable_C"))
        (CallFunction|RestoreCharacter)
        (Variables|Default|SetChecking_Actor 0)
        (Utilities|FlowControl|RetriggerableDelay 1.0)
        (Variables|Default|SetIs_EndChecking false)))
    (:else
      (if (and (not (Variables|Default|GetIs_EndChecking)) (not (Variables|Default|GetIs_StartChecking)))
        (bind _detected_actor (Variables|/Game/Game/Blueprints/Components/AC_Interact.AC_Interact_C|GetDetected_Actor (Actor|GetComponentbyClass (CallFunction|GetBPCharacter) "/Game/Game/Blueprints/Components/AC_Interact.AC_Interact_C"))
          (:then
            (Utilities|IsValid (Actor|GetComponentbyClass _detected_actor "/Game/Game/Blueprints/Components/AC_Checkable.AC_Checkable_C")
              (:Is%20Valid
                (Variables|Default|SetChecking_Actor _detected_actor)
                (Variables|Default|SetIs_StartChecking true)
                (CallFunction|SetCharacterPlayerState "NewEnumerator0")
                (Default|StartChecking (Actor|GetComponentbyClass _detected_actor "/Game/Game/Blueprints/Components/AC_Checkable.AC_Checkable_C"))
                (Utilities|FlowControl|RetriggerableDelay 1.0)
                (Variables|Default|SetIs_StartChecking false))))
          (:else))))))

(event EventBeginPlay)

(event EventTick
  (params (DeltaSeconds :type Float%20%28single-precision%29)))

(fn RestoreCharacter
  (bind _bp_character (CallFunction|GetBPCharacter))
  (bind _childactor_checkingobject (Variables|/Game/Game/Blueprints/BP_Character.BP_Character_C|GetChildActor_CheckingObject _bp_character))
  (CallFunction|SetCharacterPlayerState "NewEnumerator2")
  ;[1 1 1] 还原
  (Transformation|SetRelativeRotation _childactor_checkingobject "0, 0, 0" false false)
  (Transformation|SetRelativeScale3D _childactor_checkingobject "1.000000,1.000000,1.000000"))