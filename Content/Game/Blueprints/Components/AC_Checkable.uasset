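; AC_Checkable is an actor component that lets its owner be inspected up close.
; Start_Checking hides the owner, spawns a BP_CheckingObject with the owner's static mesh, or flies the existing one to the camera, and shows a WB_CheckObject widget.
; End_Checking sends the proxy back, removes the widget and unhides the owner after a short delay.
; The proxy is reused across inspections and cleaned up with the widget on EndPlay.
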(event Custom|Start_Checking
  (CallFunction|HideActor (Components|GetOwner) true)
  (Utilities|IsValid (Variables|Default|GetCheckingObject)
    (:Is%20Valid
      (Default|FlytoCamera (Variables|Default|GetCheckingObject)))
    (:Is%20Not%20Valid
      ;[1 1 1] Spawn_CheckingObject
      (bind _returnvalue (Game|SpawnActorfromClass "/Game/Game/UI/InGame/BP_CheckingObject.BP_CheckingObject_C" (Transformation|GetActorTransform (Components|GetOwner)) "AlwaysSpawn" "MultiplyWithRoot" 0 (Variables|/Script/Engine.StaticMeshComponent|GetStaticMesh (Actor|GetComponentbyClass (Components|GetOwner) "/Script/Engine.StaticMeshComponent")) 0))
      (Variables|Default|SetCheckingObject _returnvalue)))
  ;[1 1 1] Create_CheckingUI
  (bind _returnvalue_2 (UserInterface|CreateWidget "/Game/Game/UI/InGame/WB_CheckObject.WB_CheckObject_C" 0 (Components|GetOwner)))
  (bind _output_get (Variables|Default|SetWB_CheckObject _returnvalue_2))
  (UserInterface|Viewport|AddtoViewport _output_get 0))

(event Custom|End_Checking
  (Utilities|IsValid (Variables|Default|GetCheckingObject)
    (:Is%20Valid
      (Default|BacktoPosition (Variables|Default|GetCheckingObject))
      (Widget|RemovefromParent (Variables|Default|GetWB_CheckObject))
      (Utilities|FlowControl|Delay 1.0)
      (CallFunction|HideActor (Components|GetOwner) false))))

(event EventBeginPlay)

(event EventEndPlay
  (params (EndPlayReason :type EEndPlayReason%20Enum :default "Destroyed"))
  (bind _wb_checkobject (Variables|Default|GetWB_CheckObject)
    (:then
      (Widget|RemovefromParent _wb_checkobject))
    (:else
      _))
  (bind _checkingobject (Variables|Default|GetCheckingObject)
    (:then
      (Actor|DestroyActor _checkingobject))
    (:else)))