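; Interaction component that lets its owning character detect and use objects with an AC_Interactable component.
; Each Tick, a short object-type line trace from the owner's camera stores the hit actor and shows its hint.
; A hit flagged as triggered switches the player state to Interacting Triggered, otherwise the state is set to Default.
; The Interact event calls CallOnInteract on the detected actor's interactable component.
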(event Custom|Interact
  (bind _detected_actor (Variables|Default|GetDetected_Actor)
    (:then
      (Default|CallOnInteract (Actor|GetComponentbyClass _detected_actor "/Game/Game/Blueprints/Components/AC_Interactable.AC_Interactable_C")))
    (:else)))

(event EventBeginPlay)

(event EventTick
  (params (DeltaSeconds :type Float%20%28single-precision%29))
  (switch Utilities|FlowControl|Switch|SwitchonE_PlayerState (CallFunction|GetCharacterPlayerState)
    (:NewEnumerator2
      _)
    (:NewEnumerator3
      _))
  (bind _hitactor (CallFunction|DetectItem))
  (Utilities|IsValid _hitactor
    (:Is%20Valid
      (Variables|Default|SetDetected_Actor _hitactor)
      (Default|ShowHint (Actor|GetComponentbyClass _hitactor "/Game/Game/Blueprints/Components/AC_Interactable.AC_Interactable_C"))
      (if (Variables|/Game/Game/Blueprints/Components/AC_Interactable.AC_Interactable_C|GetIs_Triggered_Interact (Actor|GetComponentbyClass _hitactor "/Game/Game/Blueprints/Components/AC_Interactable.AC_Interactable_C"))
        (CallFunction|SetCharacterPlayerState "NewEnumerator3")
        (else
          (CallFunction|SetCharacterPlayerState "NewEnumerator2" :!label _label))))
    (:Is%20Not%20Valid
      (Variables|Default|SetDetected_Actor 0)
      (goto _label))))

(fn DetectItem
  (bind _returnvalue (Components|GetOwner))
  (bind _returnvalue_2 (Actor|GetComponentbyClass _returnvalue "/Script/Engine.CameraComponent"))
  (bind _returnvalue_3 (Transformation|GetWorldLocation _returnvalue_2))
  (bind _outhit (Collision|LineTraceForObjects _returnvalue_3 (+ _returnvalue_3 (* (Math|Vector|GetForwardVector _returnvalue_2) 300)) (Utilities|Array|MakeArray "ObjectTypeQuery7") false 0 "None"))
  (return (.HitActor (Collision|BreakHitResult _outhit))))