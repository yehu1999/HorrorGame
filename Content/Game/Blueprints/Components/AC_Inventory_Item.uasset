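; Inventory item component that keeps the character's items as an array of row name and amount entries.
; AddItem searches the array for a matching row name and adds to that entry's amount, or appends a new entry when none matches.
; Each add then calls the owning character's player profile save.
; BeginPlay is empty, and an AddItem call in the event graph is unconnected.
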(event EventBeginPlay)

(fn AddItem
  (params (InventoryContent :type S%20Inventory%20Content%20Structure))
  (bind (_rowname _amount) (Utilities|Struct|BreakS_InventoryContent InventoryContent))
  (LocalVariables|SetLocal_Is_FoundContent false)
  (bind _array_element (Utilities|Array|ForEachLoopwithBreak (Variables|Default|GetInventory) :!label _label)
    (:LoopBody
      (if (== (.RowName (Utilities|Struct|BreakS_InventoryContent _array_element)) _rowname)
        (Utilities|Struct|SetmembersinS_InventoryContent _array_element (+ (.Amount (Utilities|Struct|BreakS_InventoryContent _array_element)) _amount))
        (LocalVariables|SetLocal_Is_FoundContent true)
        (goto _label Break)))
    (:Completed
      (if (LocalVariables|GetLocal_Is_FoundContent)
        _
        (else
          (Utilities|Array|Add (Variables|Default|GetInventory) InventoryContent)))
      (Default|CharacterSaveGamePlayerProfile (CallFunction|GetBPCharacter)))))