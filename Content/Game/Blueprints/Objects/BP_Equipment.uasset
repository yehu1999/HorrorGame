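; BP_Equipment is a world pickup that gives the player a piece of equipment when interacted with.
; On interact, it adds its InventoryContent row name to the character's ACInventoryEquipment and removes itself from the level save record.
; It then destroys its directly attached actors and itself, and finally calls ChangeEquipment to switch the character to the new item.
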(event OnInteract(AC_Interactable)
  (bind _bp_character (CallFunction|GetBPCharacter))
  (bind _inventorycontent (Variables|Default|GetInventoryContent))
  (bind _rowname (Utilities|Struct|BreakS_InventoryContent _inventorycontent))
  (bind _ac_inventory_equipment (Variables|/Game/Game/Blueprints/BP_Character.BP_Character_C|GetAC_Inventory_Equipment _bp_character))
  (Default|AddNewEquipment _ac_inventory_equipment _rowname)
  (CallFunction|RemovefromLevelSG) ; 从存档记录中删去
  (for _array_element (Actor|GetAttachedActors true false)
    (Actor|DestroyActor _array_element))
  (Actor|DestroyActor)
  (Default|ChangeEquipment _ac_inventory_equipment _rowname))

(event EventBeginPlay
  (|CallParentFunction) ; 此节点被禁用，将不会被调用。\n从引脚连出引线来编译功能。
)

(event Collision|EventActorBeginOverlap
  (params (OtherActor :type Actor%20Object%20Reference)))

(event EventTick
  (params (DeltaSeconds :type Float%20%28single-precision%29)))

(fn ConstructionScript
  (|CallParentFunction))