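; BP_Item is a pickup object that moves its InventoryContent into the character's inventory when interacted with.
; The AC_Interactable component's OnInteract event passes the content to AddItem on the character's ACInventoryItem component.
; It then destroys its directly attached actors, without recursing into their children, and finally itself.
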(event OnInteract(AC_Interactable)
  (Default|AddItem (Variables|/Game/Game/Blueprints/BP_Character.BP_Character_C|GetAC_Inventory_Item (CallFunction|GetBPCharacter)) (Variables|Default|GetInventoryContent))
  (for _array_element (Actor|GetAttachedActors true false)
    (Actor|DestroyActor _array_element))
  (Actor|DestroyActor))

(event EventBeginPlay
  (|CallParentFunction) ; 此节点被禁用，将不会被调用。\n从引脚连出引线来编译功能。
)

(fn ConstructionScript
  (|CallParentFunction))