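; BP_Object is a data-driven world object whose appearance and identity come from the DT_Object data table.
; The construction script looks up the row named by InventoryContent.RowName and applies its mesh and object type, so placed instances update in the editor.
; GetCheckingData reads the same row to return the object's name and description.
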(event EventBeginPlay)

(fn ConstructionScript
  (bind _returnvalue (Utilities|GetDataTableRow "/Game/Game/Data/DT_Object.DT_Object" (.RowName (Utilities|Struct|BreakS_InventoryContent (Variables|Default|GetInventoryContent))))
    (:then
      (Components|StaticMesh|SetStaticMesh (Variables|Default|GetStaticMesh) (.Mesh (Utilities|Struct|BreakS_Object _returnvalue)))
      (Variables|Default|SetObject%20Type (.ObjectType (Utilities|Struct|BreakS_Object _returnvalue))))))

(fn GetCheckingData
  (bind _returnvalue (Utilities|GetDataTableRow "/Game/Game/Data/DT_Object.DT_Object" (.RowName (Utilities|Struct|BreakS_InventoryContent (Variables|Default|GetInventoryContent))))
    (:then
      (return (.Name (Utilities|Struct|BreakS_Object _returnvalue)) (.Description (Utilities|Struct|BreakS_Object _returnvalue))))))