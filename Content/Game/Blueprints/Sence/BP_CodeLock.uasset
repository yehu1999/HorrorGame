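; BP_CodeLock is a keypad code lock that unlocks a linked BP_Door when the entered code matches.
; The construction script gathers digit, Enter and Reset BP_Button child actors, whose press events BeginPlay binds to one handler.
; BeginPlay also creates the WB_CodeScreen slots and trims Code to CodeLength, deferred until child components exist.
; Digits update screen and input string, Reset clears both, and Enter does nothing on a mismatch.
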(event Custom|InputCode_Lock
  (params (String :type String))
  (bind _widget_codescreen (Variables|Default|GetWidget_CodeScreen))
  (bind _returnvalue (UserInterface|GetWidget _widget_codescreen))
  (bind _aswb_code_screen (Utilities|Casting|CastToWB_CodeScreen _returnvalue))
  (Utilities|IsValid _aswb_code_screen
    (:Is%20Valid
      (Default|InputCodeScreen _aswb_code_screen String)
      (Variables|Default|SetInput (Utilities|String|Append (Variables|Default|GetInput) String)))))

(event Custom|ButtonPressed
  (params (Button_Content :type String))
  (switch string Button_Content
    (:Default
      (CallFunction|InputCodeLock Button_Content))
    (:Enter
      (CallFunction|EnterCode))
    (:Reset
      (CallFunction|ResetCode))))

(event Custom|EnterCode
  (if (Utilities|Enum|Equal(Enum) (Variables|Default|GetInput) (Variables|CodeLock|GetCode))
    (Default|UnlockDoor (Variables|CodeLock|GetBP_Door))))

(event Custom|ResetCode
  (bind _widget_codescreen (Variables|Default|GetWidget_CodeScreen))
  (bind _returnvalue (UserInterface|GetWidget _widget_codescreen))
  (bind _aswb_code_screen (Utilities|Casting|CastToWB_CodeScreen _returnvalue))
  (Utilities|IsValid _aswb_code_screen
    (:Is%20Valid
      (Default|ResetCodeScreen _aswb_code_screen)
      (Variables|Default|SetInput ""))))

(event EventBeginPlay
  (bind _code_length (Variables|CodeLock|GetCode_Length))
  (Utilities|FlowControl|Sequence
    (:then_0
      (bind _aswb_code_screen (Utilities|Casting|CastToWB_CodeScreen (UserInterface|GetWidget (Variables|Default|GetWidget_CodeScreen))))
      (Default|CreateCodeSlot _aswb_code_screen _code_length)
      (Variables|CodeLock|SetCode (Utilities|String|GetSubstring (Variables|CodeLock|GetCode) 0 _code_length)))
    (:then_1
      (for _array_element (Variables|Default|GetArray_Button)
        (EventDispatchers|BindEventtoOnBPButtonPressed _array_element (delegate Custom|ButtonPressed))))))

(event EventTick
  (params (DeltaSeconds :type Float%20%28single-precision%29)))

(fn ConstructionScript
  (Variables|Default|SetArray_Button (Utilities|Array|MakeArray (.AsBP%20Button (Utilities|Casting|CastToBP_Button (Variables|/Script/Engine.ChildActorComponent|GetChildActor (Variables|Default|GetChildActor_Button_0)))) (.AsBP%20Button (Utilities|Casting|CastToBP_Button (Variables|/Script/Engine.ChildActorComponent|GetChildActor (Variables|Default|GetChildActor_Button_1)))) (.AsBP%20Button (Utilities|Casting|CastToBP_Button (Variables|/Script/Engine.ChildActorComponent|GetChildActor (Variables|Default|GetChildActor_Button_2)))) (.AsBP%20Button (Utilities|Casting|CastToBP_Button (Variables|/Script/Engine.ChildActorComponent|GetChildActor (Variables|Default|GetChildActor_Button_3)))) (.AsBP%20Button (Utilities|Casting|CastToBP_Button (Variables|/Script/Engine.ChildActorComponent|GetChildActor (Variables|Default|GetChildActor_Button_4)))) (.AsBP%20Button (Utilities|Casting|CastToBP_Button (Variables|/Script/Engine.ChildActorComponent|GetChildActor (Variables|Default|GetChildActor_Button_5)))) (.AsBP%20Button (Utilities|Casting|CastToBP_Button (Variables|/Script/Engine.ChildActorComponent|GetChildActor (Variables|Default|GetChildActor_Button_6)))) (.AsBP%20Button (Utilities|Casting|CastToBP_Button (Variables|/Script/Engine.ChildActorComponent|GetChildActor (Variables|Default|GetChildActor_Button_7)))) (.AsBP%20Button (Utilities|Casting|CastToBP_Button (Variables|/Script/Engine.ChildActorComponent|GetChildActor (Variables|Default|GetChildActor_Button_8)))) (.AsBP%20Button (Utilities|Casting|CastToBP_Button (Variables|/Script/Engine.ChildActorComponent|GetChildActor (Variables|Default|GetChildActor_Button_9)))) (.AsBP%20Button (Utilities|Casting|CastToBP_Button (Variables|/Script/Engine.ChildActorComponent|GetChildActor (Variables|Default|GetChildActor_Button_Enter)))) (.AsBP%20Button (Utilities|Casting|CastToBP_Button (Variables|/Script/Engine.ChildActorComponent|GetChildActor (Variables|Default|GetChildActor_Button_Reset)))))))