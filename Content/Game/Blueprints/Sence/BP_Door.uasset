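; Interactable door that the player swings by horizontal mouse movement, clamped between min and max yaw.
; A dot product of the flattened player-to-door and arrow vectors, optionally reversed, finds the player's side and sets the mouse sign.
; In one swing direction per side, an optional box trace blocks rotation into a Character-tagged pawn.
; When locked it plays a can't-open sound; Unlock_Door clears the lock and re-enables the interact component's trigger flag.
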(event OnInteract(AC_Interactable)
  (bind _bp_playercontroller (CallFunction|GetBPPlayerController))
  (bind _bp_character (CallFunction|GetBPCharacter))
  (bind _self self)
  (bind _arrow (Variables|Default|GetArrow))
  (bind _mousex (Default|GetControllerMouseXY _bp_playercontroller))
  (bind _returnvalue (Transformation|GetActorLocation _bp_character))
  (bind _returnvalue_2 (Transformation|GetActorLocation _self))
  (bind _returnvalue_3 (Math|Vector|GetForwardVector _arrow))
  (bind _returnvalue_4 (Math|Vector|MakeVector (.x _returnvalue_3) (.y _returnvalue_3) 0.0))
  (bind _returnvalue_5 (- _returnvalue_2 _returnvalue))
  (bind _returnvalue_6 (Math|Vector|MakeVector (.x _returnvalue_5) (.y _returnvalue_5) 0.0))
  (bind _returnvalue_7 (Math|Vector|DotProduct _returnvalue_6 _returnvalue_4))
  (bind _returnvalue_8 (> _returnvalue_7 0.0))
  (if (Variables|Door|GetIs_Locked)
    (Audio|PlaySoundatLocation "/Game/Assets/Aduios/SFX/Door_CantOpen.Door_CantOpen" (Transformation|GetActorLocation) "0, 0, 0" 1.0 1.0 0.0 0 0 0 0)
    (else
      (if (Variables|Door|GetIs_DirectionReverse)
        (Variables|Default|SetIs_FaceToDoor (not _returnvalue_8))
        (else
          (Variables|Default|SetIs_FaceToDoor _returnvalue_8)))
      ;[1 1 1] 判断门打开的方向
      (if (Variables|Default|GetIs_FaceToDoor)
        (bind _output_get (Variables|Default|SetDelta_Rotation (* _mousex -6.0)))
        (if (> _output_get 0.0)
          (Transformation|SetRelativeRotation (Variables|Default|GetStaticMesh) (Math|Rotator|MakeRotator 0.0 0.0 (Math|Float|Clamp(Float) (.yaw (Math|Rotator|CombineRotators (Math|Rotator|MakeRotator 0.0 0.0 (.yaw (Variables|/Script/Engine.SceneComponent|GetRelativeRotation (Variables|Default|GetStaticMesh)))) (Math|Rotator|MakeRotator 0.0 0.0 (Variables|Default|GetDelta_Rotation)))) (Variables|Door|GetMin_Rotation) (Variables|Door|GetMax_Rotation))) false false :!label _label)
          (else
            (if (Variables|Door|GetIs_DetectDoorCollision) :!label _label_2
              (bind _has_hitcharacter (CallFunction|DetectDoorCollision))
              (if (not _has_hitcharacter)
                (goto _label))
              (else
                (goto _label)))))
        (else
          (bind _output_get_2 (Variables|Default|SetDelta_Rotation (* _mousex 6.0)))
          (if (< _output_get_2 0.0)
            (goto _label)
            (else
              (goto _label_2))))))))

(event Custom|Unlock_Door
  (Variables|Door|SetIs_Locked false)
  (Audio|PlaySoundatLocation "/Game/Assets/Aduios/SFX/Door_LockOpen.Door_LockOpen" (Transformation|GetActorLocation) "0, 0, 0" 1.0 1.0 0.0 0 0 0 0)
  (Variables|/Game/Game/Blueprints/Components/AC_Interactable.AC_Interactable_C|SetIs_Triggered_Interact (Variables|Default|GetAC_Interactable) true))

(event EventBeginPlay)

(event EventTick
  (params (DeltaSeconds :type Float%20%28single-precision%29)))

(fn ConstructionScript
  (bind _ac_interactable (Variables|Default|GetAC_Interactable))
  (if (Variables|Door|GetIs_Locked)
    (Variables|/Game/Game/Blueprints/Components/AC_Interactable.AC_Interactable_C|SetIs_Triggered_Interact _ac_interactable false)
    (else
      (Variables|/Game/Game/Blueprints/Components/AC_Interactable.AC_Interactable_C|SetIs_Triggered_Interact _ac_interactable true))))

(fn DetectDoorCollision
  (bind _box (Variables|Default|GetBox))
  (bind _returnvalue (Transformation|GetWorldLocation _box))
  (bind (_outhit _returnvalue_2) (Class|KismetSystemLibrary|BoxTraceSingleforObjects _returnvalue _returnvalue "30.000000,45.000000,113.000000" (Variables|/Script/Engine.SceneComponent|GetRelativeRotation (Variables|Default|GetStaticMesh)) (Utilities|Array|MakeArray "ObjectTypeQuery3") false 0 "None" true "(R=1.000000,G=0.000000,B=0.000000,A=1.000000)" "(R=0.000000,G=1.000000,B=0.000000,A=1.000000)" 1.0))
  (if _returnvalue_2
    (return (Actor|ActorHasTag (.HitActor (Collision|BreakHitResult _outhit)) "Character"))
    (else
      (return false))))