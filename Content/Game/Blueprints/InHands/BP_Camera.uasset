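; BP_Camera is a handheld item that works as a toggleable flashlight, despite its name.
; AC_InHandable Equip and Unequip events show or hide the character's ChildActorBPCamera, while Use toggles the SpotLight with a sound when equipped and usable.
; A breakdown event disables further use and, if the light is on, plays a timeline that scales its intensity.
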(event Use(AC_InHandable)
  (if (and (Variables|Default|GetIs_Equipped) (Variables|Default|GetIs_Usable))
    (bind _output_get (Variables|Default|SetIs_TurnOn (not (Variables|Default|GetIs_TurnOn))))
    (if _output_get
      (Rendering|Components|Light|SetIntensity (Variables|Default|GetSpotLight) (Variables|Default|GetLightIntensity_TurnOn))
      (else
        (Rendering|Components|Light|SetIntensity (Variables|Default|GetSpotLight) 0.0)))
    (Audio|PlaySoundatLocation "/Game/Assets/Aduios/SFX/FlashLight_TurnOn.FlashLight_TurnOn" (Transformation|GetActorLocation) "0, 0, 0" 1.0 1.0 0.0 0 0 0 0)))

(event Equip(AC_InHandable)
  (bind _output_get (Variables|Default|SetIs_Equipped true))
  (Rendering|SetVisibility (Variables|/Game/Game/Blueprints/BP_Character.BP_Character_C|GetChildActor_BP_Camera (CallFunction|GetBPCharacter)) _output_get true))

(event Unequip(AC_InHandable)
  (bind _output_get (Variables|Default|SetIs_Equipped false))
  (Rendering|SetVisibility (Variables|/Game/Game/Blueprints/BP_Character.BP_Character_C|GetChildActor_BP_Camera (CallFunction|GetBPCharacter)) _output_get true))

(event Custom|FlashLight_Breakdown
  (Variables|Default|SetIs_Usable false)
  (if (Variables|Default|GetIs_TurnOn)
    (bind _light_percent (Timeline|Timeline_FlashLight_Breakdown Play)
      (:Update
        (Rendering|Components|Light|SetIntensity (Variables|Default|GetSpotLight) (* _light_percent (Variables|Default|GetLightIntensity_TurnOn)))))))

(event EventBeginPlay)

(event EventTick
  (params (DeltaSeconds :type Float%20%28single-precision%29)))

(fn ConstructionScript)